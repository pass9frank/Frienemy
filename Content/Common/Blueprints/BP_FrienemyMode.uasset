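; BP_FrienemyMode is a game mode that gives joining players asymmetric roles: one Guardian and any number of Guys.
; The first login randomly picks which of the first two players becomes the Guardian and caches all PlayerStart actors.
; Each login spawns and possesses the role's pawn, with Guys cycling through the start points.
; It records the spawned pawns and activates a different virtual joystick layout per role.
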(event `self.ReceiveBeginPlay`)

(event `self.K2_PostLogin`
  (params (NewPlayer :type "PlayerController Object Reference"))
  (bind _startlocations (`self.StartLocations`))
  (`|ExecutionSequence`
    (:`then_0`
      (if (== (`self.GuardianIndex`) -1)
        (set `self.GuardianIndex` (`KismetMathLibrary.RandomInteger` 2))
        (bind _outactors (`GameplayStatics.GetAllActorsOfClass` "/Script/Engine.PlayerStart"))
        (set `self.StartLocations` _outactors)))
    (:`then_1`
      (if (== (`self.PlayerIndex`) (`self.GuardianIndex`))
        (bind _returnvalue (`|SpawnActorFromClass` "/Game/Common/Blueprints/BP_Guardian.BP_Guardian_C" (`KismetMathLibrary.MakeTransform` (0.0 0.0 0.0)) "Undefined" "OverrideRootScale" null null))
        (`Controller.Possess` NewPlayer _returnvalue)
        (set `self.Guardian` _returnvalue)
        (`self.EnableInput` _returnvalue NewPlayer)
        (`PlayerController.ActivateTouchInterface` NewPlayer "/Game/JoyStick/HUD/LeftVirtualJoystickOnly.LeftVirtualJoystickOnly")
        (else
          (bind _returnvalue_2 (`|SpawnActorFromClass` "/Game/Characters/BaseCharacter/BP_Guy.BP_Guy_C" (`self.GetTransform` (`|GetArrayItem` _startlocations (mod (`self.PlayerIndex`) (`KismetArrayLibrary.Array_Length` _startlocations)))) "Undefined" "OverrideRootScale" NewPlayer null))
          (`Controller.Possess` NewPlayer _returnvalue_2)
          (`KismetArrayLibrary.Array_Add` (`self.Guys`) _returnvalue_2)
          (`self.EnableInput` _returnvalue_2 NewPlayer)
          (`PlayerController.ActivateTouchInterface` NewPlayer "/Game/JoyStick/HUD/DefaultVirtualJoysticks.DefaultVirtualJoysticks")))
      (`/Engine/EditorBlueprintResources/StandardMacros.IncrementInt` (`self.PlayerIndex`)))))

(fn `UserConstructionScript`)