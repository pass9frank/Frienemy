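; BP_Guardian is a touch-controlled shooter that launches BP_Ball actors using a press, drag and release gesture.
; A first-finger press traces one custom channel to set the aim flag and start location.
; Release deprojects the screen point and traces a second channel, spawning a ball at the start, rotated toward the hit, if aiming.
; Drag hits feed an empty Aim event, and each phase draws colored debug points.
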(event `AimStart`
  (params (AimStartLoc :type "Vector Structure"))
  (set `self.AimStartLoc` AimStartLoc))

(event `Aim`
  (params (AimLoc :type "Vector Structure")))

(event `Shoot`
  (params (LastLoc :type "Vector Structure"))
  (bind _aimstartloc (`self.AimStartLoc`))
  (if (`self.bIsAim`)
    (`|SpawnActorFromClass` "/Game/Common/Blueprints/BP_Ball.BP_Ball_C" (`KismetMathLibrary.MakeTransform` _aimstartloc (`KismetMathLibrary.FindLookAtRotation` _aimstartloc LastLoc)) "Undefined" "OverrideRootScale" null null)))

(event `InputTouch`
  (params (Location :type "Vector Structure") (FingerIndex :type "ETouchIndex Enum"))
  (bind _returnvalue (`GameplayStatics.GetPlayerController` 0))
  (bind (_hitresult _returnvalue_2) (`PlayerController.GetHitResultUnderFingerByChannel` _returnvalue "Touch1" "TraceTypeQuery4" false))
  (bind (_worldposition _worlddirection) (`GameplayStatics.DeprojectScreenToWorld` _returnvalue (`KismetMathLibrary.MakeVector2D` (.x Location) (.y Location))))
  (bind (_hitresult_2 _returnvalue_3) (`PlayerController.GetHitResultUnderFingerByChannel` _returnvalue "Touch1" "TraceTypeQuery3" false))
  (bind (_bblockinghit _binitialoverlap _time _distance _location) (`GameplayStatics.BreakHitResult` _hitresult_2))
  (bind (_bblockinghit_2 _binitialoverlap_2 _time_2 _distance_2 _location_2) (`GameplayStatics.BreakHitResult` _hitresult))
  (:`Pressed`
    (switch `ETouchIndex` FingerIndex
      (:`Touch1`
        (set `self.bIsAim` _returnvalue_3)
        (if _returnvalue_3
          (`self.AimStart` _location)
          (`KismetSystemLibrary.DrawDebugPoint` _location 20.0 (struct :`R` 0.973958 :`B` 0.315982 :`A` 1.0) 5.0)))))
  (:`Released`
    (switch `ETouchIndex` FingerIndex
      (:`Touch1`
        (bind (_outhit _returnvalue_4) (`KismetSystemLibrary.LineTraceSingle` _worldposition (+ _worldposition (* _worlddirection 10000.0)) "TraceTypeQuery4"))
        (if _returnvalue_4
          (bind (_bblockinghit_3 _binitialoverlap_3 _time_3 _distance_3 _location_3) (`GameplayStatics.BreakHitResult` _outhit))
          (`self.Shoot` _location_3)
          (`KismetSystemLibrary.DrawDebugPoint` _location_3 20.0 (struct :`G` 0.068233 :`B` 0.973958 :`A` 1.0) 5.0)))))
  (:`Moved`
    (if _returnvalue_2
      (`self.Aim` _location_2)
      (`KismetSystemLibrary.DrawDebugPoint` _location_2 5.0 (struct :`G` 0.973958 :`B` 0.323298 :`A` 1.0) 1.0))))

(fn `UserConstructionScript`)