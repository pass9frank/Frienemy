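; Game instance for Frienemy that manages the front-end menus for login, room list and room creation.
; Login validates credentials by scanning every UserTable data table row for a matching username and password.
; Each Show function lazily creates and caches its widget, resetting the login and creation screens on reuse and updating sessions for the room list.
; ShowTargetUI keeps one menu visible, removing the others and setting UI-only input with the cursor shown.
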(fn `Login`
  (params (UserName :type String) (Password :type String))
  (returns (bIsSuccess :type Boolean))
  (bind _outrownames (`DataTableFunctionLibrary.GetDataTableRowNames` "/Game/Data/UserTable.UserTable"))
  (for _array_element _outrownames
    (bind _returnvalue (`|GetDataTableRow` "/Game/Data/UserTable.UserTable" _array_element)
      (:`then`
        (bind (_username _nickname _password) (break `/Game/Data/UserInfo` _returnvalue))
        (if (and (`KismetStringLibrary.EqualEqual_StrStr` Password _password) (`KismetStringLibrary.EqualEqual_StrStr` _username UserName))
          (return true)))))
  (return false))

(fn `ShowLogin`
  (bind _ui_login (`self.UI_Login`))
  (`/Engine/EditorBlueprintResources/StandardMacros.IsValid` _ui_login
    (:`Is Valid`
      (`/Game/UI/UILevel/Blueprints/UMG_Login.Reset` _ui_login))
    (:`Is Not Valid`
      (bind _returnvalue (`|CreateWidget` "/Game/UI/UILevel/Blueprints/UMG_Login.UMG_Login_C" (`GameplayStatics.GetPlayerController` 0)))
      (set `self.UI_Login` _returnvalue)))
  (`self.ShowTargetUI` _ui_login))

(fn `ShowRoomCreate`
  (bind _ui_roomcreate (`self.UI_RoomCreate`))
  (`/Engine/EditorBlueprintResources/StandardMacros.IsValid` _ui_roomcreate
    (:`Is Valid`
      (`/Game/UI/UILevel/Blueprints/UMG_RoomCreate.Reset` _ui_roomcreate))
    (:`Is Not Valid`
      (bind _returnvalue (`|CreateWidget` "/Game/UI/UILevel/Blueprints/UMG_RoomCreate.UMG_RoomCreate_C" (`GameplayStatics.GetPlayerController` 0)))
      (set `self.UI_RoomCreate` _returnvalue)))
  (`self.ShowTargetUI` _ui_roomcreate))

(fn `ShowRoomList`
  (bind _ui_roomlist (`self.UI_RoomList`))
  (`/Engine/EditorBlueprintResources/StandardMacros.IsValid` _ui_roomlist
    (:`Is Valid`
      _)
    (:`Is Not Valid`
      (bind _returnvalue (`|CreateWidget` "/Game/UI/UILevel/Blueprints/UMG_RoomList.UMG_RoomList_C" (`GameplayStatics.GetPlayerController` 0)))
      (bind _output_get (set `self.UI_RoomList` _returnvalue))))
  (`self.ShowTargetUI` _output_get)
  (`/Game/UI/UILevel/Blueprints/UMG_RoomList.UpdateSessions` _ui_roomlist))

(fn `ShowTargetUI`
  (params (TargetWidget :type "UserWidget Object Reference"))
  (locals (tmpWidgets :type "Array of UserWidget Object Reference"))
  (bind _returnvalue (`GameplayStatics.GetPlayerController` 0))
  (bind _output_get (set `local.tmpWidgets` (`|MakeArray` (`self.UI_Login`) (`self.UI_RoomList`) (`self.UI_RoomCreate`) :!type "UserWidget Object Reference")))
  (bind _returnvalue_2 (`KismetArrayLibrary.Array_RemoveItem` _output_get TargetWidget))
  (if _returnvalue_2
    (for _array_element (`local.tmpWidgets`)
      (`/Engine/EditorBlueprintResources/StandardMacros.IsValid` _array_element
        (:`Is Valid`
          (`Widget.RemoveFromParent` _array_element))))
    (`UserWidget.AddToViewport` TargetWidget 0)
    (`WidgetBlueprintLibrary.SetInputMode_UIOnlyEx` _returnvalue TargetWidget)
    (set `PlayerController.bShowMouseCursor` true _returnvalue)))